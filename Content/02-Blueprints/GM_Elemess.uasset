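; Game mode for Elemess's local two-player EarthBender arena, running timed rounds toward a match winner.
; BeginPlay creates the second player, plays an intro sequence, spawns rocks at spawners and starts a countdown widget.
; Tick polls health, fall height and timer; a round end checks for a winner, otherwise adds a point and reloads the arena.
; Scores persist in BP_GameInstance across reloads; match end only prints messages.
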(event Custom|StartCountDownTime
  ;[0.5432 0.4965 1] TIMER
  (CallFunction|SubstractTimer)
  (Utilities|Time|SetTimerbyEvent (delegate Custom|CountDownTimer) 1.0 true))

(event Custom|CountDownTimer
  ;[0.5432 0.4965 1] TIMER
  (bind _foundwidgets (Widget|GetAllWidgetsOfClass "/Game/02-Blueprints/01-UI/Widget/WB_Timer.WB_Timer_C" true))
  (Default|UpdateTimer (Utilities|Array|Get(acopy) _foundwidgets) (Variables|Default|Getminutes) (Variables|Default|Getseconds))
  (Variables|Default|Setseconds (- (Variables|Default|Getseconds) 1))
  (if (< (Variables|Default|Getseconds) 0)
    (if (not (== (Variables|Default|Getminutes) 0))
      (Variables|Default|Setminutes (- (Variables|Default|Getminutes) 1))
      (Variables|Default|Setseconds 59))))

(event Custom|Change%20Level
  ;[0.6678 1 0.7297] Change Level
  (Game|OpenLevel(byObjectReference) "/Game/01-Maps/L_Romain_Arena.L_Romain_Arena"))

(event Custom|LocalPlayer
  ;[0.7378 0.4158 1] Create Local Player
  (bind _returnvalue (Class|GameplayStatics|CreatePlayer -1))
  (Variables|Default|SetLocal%20Player _returnvalue)
  (Utilities|FlowControl|Delay 0.5)
  (bind _outactor (Sequencer|Player|CreateLevelSequencePlayer "/Game/03-Animation/Sequencer/LS_Effector.LS_Effector"))
  (Sequencer|Player|Play (Variables|/Script/LevelSequence.LevelSequenceActor|GetSequencePlayer _outactor) :!class /Script/MovieScene.MovieSceneSequencePlayer))

(event Custom|SubstractTimer
  ;[0.5432 0.4965 1] TIMER
  (Variables|Default|Setseconds (- (Variables|Default|Getseconds) 1))
  (if (< (Variables|Default|Getseconds) 0)
    (if (not (== (Variables|Default|Getminutes) 0))
      (Variables|Default|Setminutes (- (Variables|Default|Getminutes) 1))
      (Variables|Default|Setseconds 59))))

(event Custom|TimerEnd
  ;[1 0.7999 0.9288] Conditions de victoire
  ;;[1 0.9608 0.5294] Timer fini
  (if (== (Variables|Default|Getminutes) 0)
    (if (== (Variables|Default|Getseconds) 0)
      (CallFunction|WinnerCondition)
      (if (not (Variables|Default|GethaveWinner))
        (CallFunction|Reset)))))

(event Custom|CheckAndSpawnRocks
  ;[1 0.4 0.4902] Check si on peut spawn des rocks
  (bind _outactors (Actor|GetAllActorsOfClass "/Game/02-Blueprints/Stone/BP_SpawnerRock.BP_SpawnerRock_C"))
  (for _array_element _outactors
    (bind _outactors_2 (Actor|GetAllActorsOfClass "/Game/02-Blueprints/Stone/BP_Rock.BP_Rock_C"))
    (Variables|Default|SetRockFound false)
    (bind _array_element_2 (Utilities|Array|ForEachLoopwithBreak _outactors_2 :!label _label)
      (:LoopBody
        (if (< (Math|Vector|Distance(Vector) (Transformation|GetActorLocation _array_element) (Transformation|GetActorLocation _array_element_2)) 5e+02)
          (Variables|Default|SetRockFound true)
          (goto _label Break)))
      (:Completed
        (if (not (Variables|Default|GetRockFound))
          (Game|SpawnActorfromClass "/Game/02-Blueprints/Stone/BP_Rock.BP_Rock_C" (Math|Conversions|ToTransform(Vector) (Transformation|GetActorLocation _array_element)) "Undefined" "MultiplyWithRoot" 0 0))))))

(event Custom|OutArena
  ;[1 0.7999 0.9288] Conditions de victoire
  ;;[1 0.9608 0.5294] En dehors de l'arène
  (if (< (.Z (Math|Vector|BreakVector (Transformation|GetActorLocation (Variables|Default|GetPlayer1)))) 5.5e+02)
    (Default|Ragdoll (Variables|Default|GetPlayer1))
    (Variables|Default|SetPlayer1Win false)
    (Utilities|FlowControl|Delay 1.0 :!label _label)
    (CallFunction|WinnerCondition)
    (if (not (Variables|Default|GethaveWinner))
      (CallFunction|Reset))
    (elif (< (.Z (Math|Vector|BreakVector (Transformation|GetActorLocation (Variables|Default|GetPlayer2)))) 5.5e+02)
      (Default|Ragdoll (Variables|Default|GetPlayer2))
      (Variables|Default|SetPlayer1Win true)
      (goto _label))))

(event Custom|Reset
  ;[0.6588 1 0.7176] RESET LA PARTIE / LA SCENE
  (CallFunction|AddPoints)
  (Development|PrintString "Reset Level")
  (Class|GameplayStatics|RemovePlayer (Variables|Default|GetLocal%20Player) true)
  (CallFunction|ChangeLevel))

(event Custom|WinnerCondition
  ;[0.551 0.9701 1] Fin de jeu : 3 points
  (if (== (Variables|/Game/02-Blueprints/BP_GameInstance.BP_GameInstance_C|GetPlayer1Points (Variables|Default|GetGameInstance)) 2.0)
    (Development|PrintString "Player1 WIN ! ")
    (CallFunction|EndGame)
    (Variables|Default|SethaveWinner true :!label _label)
    (elif (== (Variables|/Game/02-Blueprints/BP_GameInstance.BP_GameInstance_C|GetPlayer2Points (Variables|Default|GetGameInstance)) 2.0)
      (Development|PrintString "Player2 WIN ! ")
      (CallFunction|EndGame)
      (goto _label)
      (else
        (Variables|Default|SethaveWinner false)))))

(event Custom|SpawnRock
  ;[1 0.4 0.4902] Spawn des rocks
  (bind _outactors (Actor|GetAllActorsOfClass "/Game/02-Blueprints/Stone/BP_SpawnerRock.BP_SpawnerRock_C"))
  (bind _output_get (Variables|Default|SetTargetPoints _outactors))
  (for _array_element _output_get
    (Game|SpawnActorfromClass "/Game/02-Blueprints/Stone/BP_Rock.BP_Rock_C" (Math|Conversions|ToTransform(Vector) (Transformation|GetActorLocation _array_element)) "Undefined" "MultiplyWithRoot" 0 0)))

(event Custom|NoLife
  ;[1 0.7999 0.9288] Conditions de victoire
  ;;[1 0.9608 0.5294] Plus de vie
  (if (<= (Variables|/Game/02-Blueprints/Gameplay/Characters/BP_EarthBender.BP_EarthBender_C|GetHealth (Variables|Default|GetPlayer1)) 0.0)
    (Default|Ragdoll (Variables|Default|GetPlayer1))
    (Variables|Default|SetPlayer1Win false)
    (Utilities|FlowControl|Delay 1.5 :!label _label)
    (CallFunction|WinnerCondition)
    (if (not (Variables|Default|GethaveWinner))
      (CallFunction|Reset))
    (elif (<= (Variables|/Game/02-Blueprints/Gameplay/Characters/BP_EarthBender.BP_EarthBender_C|GetHealth (Variables|Default|GetPlayer2)) 0.0)
      (Default|Ragdoll (Variables|Default|GetPlayer2))
      (Variables|Default|SetPlayer1Win true)
      (goto _label))))

(event Custom|EndGame
  ;[0.6588 1 0.7176] FIN DU JEU
  (Development|PrintString "Fin - Winner Win"))

(event Custom|Timer
  ;[0.5432 0.4965 1] TIMER
  (Utilities|FlowControl|Delay 4.0)
  (CallFunction|StartCountDownTime)
  (bind _returnvalue (UserInterface|CreateWidget "/Game/02-Blueprints/01-UI/Widget/WB_Timer.WB_Timer_C"))
  (UserInterface|Viewport|AddtoViewport _returnvalue 0))

(event EventTick
  (params (DeltaSeconds :type Float%20%28single-precision%29))
  ;[0.5051 1 0.5936] Verification des conditions à chaque temps
  (CallFunction|NoLife)
  (CallFunction|TimerEnd)
  (CallFunction|OutArena))

(event EventBeginPlay
  (Audio|PlaySound2D "/Game/04-Arts/Music/Into_Fire_Nation_Territory.Into_Fire_Nation_Territory" 1.0 1.0 0.0 0 0)
  (CallFunction|Timer)
  (bind _asbp_game_instance (Utilities|Casting|CastToBP_GameInstance (Game|GetGameInstance)))
  (Variables|Default|SetGameInstance _asbp_game_instance)
  (Development|PrintString (Utilities|String|ToString(Float) (Variables|/Game/02-Blueprints/BP_GameInstance.BP_GameInstance_C|GetPlayer1Points _asbp_game_instance)))
  (CallFunction|SpawnRock)
  (CallFunction|LocalPlayer)
  (bind _outactors (Actor|GetAllActorsOfClass "/Game/02-Blueprints/Gameplay/Characters/BP_EarthBender.BP_EarthBender_C"))
  (for (_array_element _array_index) _outactors
    (if (== _array_index 0)
      (Development|PrintString "Player 1")
      (Variables|Default|SetPlayer1 _array_element)
      (else
        (Development|PrintString "Player2")
        (Variables|Default|SetPlayer2 _array_element)))))

(fn ConstructionScript)

(fn AddPoints
  (if (Variables|Default|GetPlayer1Win)
    (Math|Float|IncrementFloat (Variables|/Game/02-Blueprints/BP_GameInstance.BP_GameInstance_C|GetPlayer1Points (Variables|Default|GetGameInstance)))
    (else
      (Math|Float|IncrementFloat (Variables|/Game/02-Blueprints/BP_GameInstance.BP_GameInstance_C|GetPlayer2Points (Variables|Default|GetGameInstance))))))