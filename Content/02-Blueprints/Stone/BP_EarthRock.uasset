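; Spinning earth rock projectile that rises from the ground, then launches along the player camera's forward direction.
; On BeginPlay a timeline lerps it from start to target position with physics and collision off, then enables both and applies a velocity-change impulse.
; A hit or the DestroyRock event prints the other actor's name, plays impact VFX and sound, then destroys the actor after a short delay.
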(event OnComponentHit(Rock)
  (params (HitComponent :type Primitive%20Component%20Object%20Reference) (OtherActor :type Actor%20Object%20Reference) (OtherComp :type Primitive%20Component%20Object%20Reference) (NormalImpulse :type Vector :default "0, 0, 0") (Hit :type Hit%20Result%20Structure%20%28by%20ref%29))
  ;[0.6892 1 0.9297] Si Collision, destruction de l'objet
  (Development|PrintString (Utilities|GetDisplayName OtherActor))
  ;;[0.7861 0.332 1] VFX SFX
  (Components|Activation|Activate (Variables|Default|GetFX_Hit) true)
  (Audio|SpawnSoundAttached "/Game/SmallSoundKit/SSKCue/MagicCue/Mgc_Glacier_Impact_01_Cue.Mgc_Glacier_Impact_01_Cue" (Variables|Default|GetRock) "None" "0, 0, 0" "0, 0, 0" "KeepRelativeOffset" false 1.0 1.0 0.0 0 0)
  (Utilities|FlowControl|Delay 0.1)
  (Actor|DestroyActor))

(event Custom|DestroyRock
  ;[0.6892 1 0.9297] Si Collision, destruction de l'objet
  (Development|PrintString (Utilities|GetDisplayName (stale OnComponentHit(Rock) OtherActor)))
  ;;[0.7861 0.332 1] VFX SFX
  (Components|Activation|Activate (Variables|Default|GetFX_Hit) true)
  (Audio|SpawnSoundAttached "/Game/SmallSoundKit/SSKCue/MagicCue/Mgc_Glacier_Impact_01_Cue.Mgc_Glacier_Impact_01_Cue" (Variables|Default|GetRock) "None" "0, 0, 0" "0, 0, 0" "KeepRelativeOffset" false 1.0 1.0 0.0 0 0)
  (Utilities|FlowControl|Delay 0.1)
  (Actor|DestroyActor))

(event EventBeginPlay
  (bind _rock (Variables|Default|GetRock))
  ;[1 0.5698 0.6196] Le disque sort du sol puis se projette vers l'avant de la caméra du joueur
  (Physics|SetSimulatePhysics (Variables|Default|GetRock) false)
  (Collision|SetCollisionEnabled (Variables|Default|GetRock) "NoCollision")
  (bind _movement (Timeline|MoveTimeLine PlayFromStart)
    (:Update
      (Transformation|SetActorLocation (Math|Vector|Lerp(Vector) (Variables|Default|GetStartPosition) (Variables|Default|GetTargetPosition) _movement) false false))
    (:Finished
      (Collision|SetCollisionEnabled _rock "QueryAndPhysics")
      (Physics|SetSimulatePhysics _rock true)
      (Physics|AddImpulse _rock (* (Math|Vector|GetForwardVector (Variables|Default|GetCameraCharacter)) 7e+03) "None" true))))

(event EventTick
  (params (DeltaSeconds :type Float%20%28single-precision%29))
  ;[0.6469 1 0.5782] Fais tourner le disque
  (Transformation|AddLocalRotation (Variables|Default|GetRock) (Math|Rotator|MakeRotator 0.0 0.0 (* DeltaSeconds 5e+01)) false false))

(fn ConstructionScript)