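; BP_EarthWall is a temporary earth wall actor that rises on spawn, sinks back down and destroys itself.
; BeginPlay and CreateEarthWall share one sequence that activates a camera shake and plays a timeline driving the Wall's Z scale.
; When the rise finishes, the timeline reverses from the end and rebinds its finished callback to DestroyEarthWall, which destroys the actor.
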(event Custom|Destroy%20EarthWall
  ;[0.1667 0.1667 0.1667] Wall Rise and Destroy Animation
  (Actor|DestroyActor))

(event Custom|Create%20EarthWall
  (bind _wall (Variables|Default|GetWall))
  (bind _tl_earthwallrise (Variables|Default|GetTL_EarthWallRise))
  (bind _returnvalue (Transformation|GetWorldScale _wall))
  ;[0.1667 0.1667 0.1667] Wall Rise and Destroy Animation
  (Components|Activation|Activate (Variables|Default|GetCameraShakeSource) true)
  (bind _height_wall (Timeline|TL_EarthWallRise PlayFromStart)
    (:Update
      (Transformation|SetWorldScale3D _wall (Math|Vector|MakeVector (.x _returnvalue) (.y _returnvalue) _height_wall)))
    (:Finished
      (Components|Timeline|ReversefromEnd _tl_earthwallrise)
      (Class|TimelineComponent|SetTimelineFinishedFunc _tl_earthwallrise (delegate Custom|Destroy%20EarthWall)))))

(event EventBeginPlay
  (bind _wall (Variables|Default|GetWall))
  (bind _tl_earthwallrise (Variables|Default|GetTL_EarthWallRise))
  (bind _returnvalue (Transformation|GetWorldScale _wall))
  ;[0.1667 0.1667 0.1667] Wall Rise and Destroy Animation
  (Components|Activation|Activate (Variables|Default|GetCameraShakeSource) true)
  (bind _height_wall (Timeline|TL_EarthWallRise PlayFromStart)
    (:Update
      (Transformation|SetWorldScale3D _wall (Math|Vector|MakeVector (.x _returnvalue) (.y _returnvalue) _height_wall)))
    (:Finished
      (Components|Timeline|ReversefromEnd _tl_earthwallrise)
      (Class|TimelineComponent|SetTimelineFinishedFunc _tl_earthwallrise (delegate Custom|Destroy%20EarthWall)))))

(fn ConstructionScript)