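; BP_Rock is a rock actor that can be destroyed and notifies the GM_Elemess game mode when it is.
; Its DestroyRock event acts only while IsOnGround is false: it activates a hit effect, plays a glacier impact sound, then destroys the actor after a brief delay.
; It then calls CheckAndSpawnRocks on the game mode, which by its name handles rock respawning.
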(event Custom|DestroyRock
  (if (not (Variables|Default|GetIsOnGround))
    (Components|Activation|Activate (Variables|Default|GetFX_Hit) true)
    (Audio|SpawnSoundAttached "/Game/SmallSoundKit/SSKCue/MagicCue/Mgc_Glacier_Impact_01_Cue.Mgc_Glacier_Impact_01_Cue" (Variables|Default|GetRock) "None" "0, 0, 0" "0, 0, 0" "KeepRelativeOffset" false 1.0 1.0 0.0 0 0)
    (Utilities|FlowControl|Delay 0.1)
    (Actor|DestroyActor)
    (bind _asgm_elemess (Utilities|Casting|CastToGM_Elemess (Game|GetGameMode)))
    (Default|CheckandSpawnRocks _asgm_elemess)))

(event Collision|EventActorBeginOverlap
  (params (OtherActor :type Actor%20Object%20Reference)))

(event EventTick
  (params (DeltaSeconds :type Float%20%28single-precision%29)))

(fn ConstructionScript)